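; Editor placement tool that scatters instanced static meshes over nearby world-static surfaces, rebuilt from its construction script.
; Construct seeds a random stream, clears old instances, then line-traces from random points within DistributionRadius along RaycastDirection, looping up to Density.
; Each hit adds an instance aligned to the impact normal with random per-axis scale.
; RadiusGizmo visualises the radius and trace distance, and RandomiseSeed rerolls the layout, optionally on every construction.
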(event EventBeginPlay)

(event Collision|EventActorBeginOverlap
  (params (OtherActor :type Actor%20Object%20Reference)))

(event EventTick
  (params (DeltaSeconds :type Float%20%28single-precision%29)))

(fn ConstructionScript
  (bind _radius_gizmo (Variables|Default|GetRadius%20Gizmo))
  (bind _distribution_radius (Variables|Distributor|GetDistribution%20Radius))
  (bind _trace_distance (Variables|Distributor|GetTrace%20Distance))
  (bind _returnvalue (/ _distribution_radius 5e+01))
  (Utilities|FlowControl|Sequence
    (:then_0
      (Transformation|SetAbsolute _radius_gizmo false false true)
      (Transformation|SetWorldScale3D _radius_gizmo (Math|Vector|MakeVector _returnvalue _returnvalue (/ _trace_distance 5e+01)))
      (Transformation|SetRelativeLocation _radius_gizmo (Math|Vector|MakeVector (/ _trace_distance 2.0) 0.0 0.0) false false))
    (:then_1
      (if (Variables|Distributor|GetRandomise%20Seed%20On%20Construction)
        (Distributor|RandomiseSeed)))
    (:then_2
      (Distributor|Construct))))

(fn RandomiseSeed
  (Variables|Distributor|SetSeed (Math|Random|RandomInteger 999999))
  (Distributor|CleanupMeshes)
  (Distributor|Construct))

(fn Construct
  (bind _returnvalue (Math|Trig|GetPI))
  (bind _returnvalue_2 (Transformation|GetActorLocation))
  (bind _random_stream (Variables|Distributor|GetRandom%20Stream))
  (bind _min_scale (Variables|Distributor|GetMin%20Scale))
  (bind _max_scale (Variables|Distributor|GetMax%20Scale))
  (bind _random_stream_2 (Variables|Distributor|GetRandom%20Stream))
  (bind _distribution_radius (Variables|Distributor|GetDistribution%20Radius))
  (bind _returnvalue_3 (Math|Random|RandomFloatinRangefromStream _min_scale _max_scale _random_stream))
  (bind _returnvalue_4 (Math|Random|RandomFloatinRangefromStream 0.0 _distribution_radius _random_stream_2))
  (bind _returnvalue_5 (/ _returnvalue 2.0))
  (bind _returnvalue_6 (* _returnvalue 2.0))
  (bind _returnvalue_7 (Math|Random|RandomFloatinRangefromStream 0.0 _returnvalue_6 _random_stream_2))
  (bind _out (CallFunction|Invert _returnvalue_5))
  (bind _returnvalue_8 (Math|Trig|Sin(Radians) _returnvalue_7))
  (bind _returnvalue_9 (Math|Random|RandomFloatinRangefromStream _out _returnvalue_5 _random_stream_2))
  (bind _returnvalue_10 (Math|Trig|Cos(Radians) _returnvalue_7))
  (bind _returnvalue_11 (Math|Trig|Cos(Radians) _returnvalue_9))
  (bind _returnvalue_12 (Math|Trig|Sin(Radians) _returnvalue_9))
  (bind _returnvalue_13 (* _returnvalue_10 _returnvalue_11 _returnvalue_4))
  (bind _returnvalue_14 (* _returnvalue_8 _returnvalue_11 _returnvalue_4))
  (bind _returnvalue_15 (* _returnvalue_12 _returnvalue_4))
  (bind _returnvalue_16 (Math|Vector|MakeVector _returnvalue_13 _returnvalue_15 _returnvalue_14))
  (bind _returnvalue_17 (+ _returnvalue_16 _returnvalue_2))
  (Math|Random|SetRandomStreamSeed (Variables|Distributor|GetRandom%20Stream) (Variables|Distributor|GetSeed))
  (Distributor|CleanupMeshes)
  (for _index (range (Class|KismetSystemLibrary|MakeLiteralInteger) (Variables|Distributor|GetDensity))
    (bind (_outhit _returnvalue_18) (Collision|LineTraceForObjects _returnvalue_17 (+ _returnvalue_17 (* (Math|Vector|GetForwardVector (Variables|Default|GetRaycast%20Direction)) (Variables|Distributor|GetTrace%20Distance))) (Utilities|Array|MakeArray "ObjectTypeQuery1") false 0 "None"))
    (if _returnvalue_18
      (Class|InstancedStaticMeshComponent|AddInstanceWorldSpace (Variables|Default|GetInstancedStaticMesh) (Math|Transform|MakeTransform (.impactpoint _outhit) (Math|Conversions|RotationFromXVector (.impactnormal _outhit)) (Math|Vector|MakeVector _returnvalue_3 _returnvalue_3 _returnvalue_3))))))

(fn CleanupMeshes
  (Components|InstancedStaticMesh|ClearInstances (Variables|Default|GetInstancedStaticMesh)))