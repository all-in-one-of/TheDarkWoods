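; BP_Entity_Base is a base entity Blueprint with a capsule and mesh that provides an optional contact drop shadow.
; The construction script places ContactShadow at the bottom of the capsule and sizes it from the larger horizontal mesh extent, scaled by ContactShadowMultiplier.
; When UseContactShadow is off, it destroys the shadow component instead.
; The event graph holds only disabled placeholder events.
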(event EventBeginPlay)

(event Collision|EventActorBeginOverlap
  (params (OtherActor :type Actor%20Object%20Reference)))

(event EventTick
  (params (DeltaSeconds :type Float%20%28single-precision%29)))

(fn ConstructionScript
  (bind _contact_shadow (Variables|Default|GetContact%20Shadow))
  (bind _contact_shadow_multiplier (Variables|Components|GetContact%20Shadow%20Multiplier))
  (bind _mesh (Variables|Character|GetMesh))
  (bind _boxextent (Collision|GetComponentBounds _mesh))
  (bind _relativelocation (Variables|/Script/Engine.SceneComponent|GetRelativeLocation _contact_shadow))
  (bind _returnvalue (Math|Float|Max(Float) (.x _boxextent) (.y _boxextent)))
  (bind _returnvalue_2 (/ _returnvalue 1e+02))
  (bind _returnvalue_3 (* _returnvalue_2 _contact_shadow_multiplier))
  (if (Variables|Components|GetUse%20Contact%20Shadow?)
    ;[1 0.4333 0.9431] Init drop shadow
    (Transformation|SetRelativeLocation _contact_shadow (Math|Vector|MakeVector (.x _relativelocation) (.y _relativelocation) (CallFunction|Invert (Components|Capsule|GetScaledCapsuleHalfHeight (Variables|Collision|GetCapsuleComponent)))) false false)
    (Transformation|SetWorldScale3D (Variables|Default|GetContact%20Shadow) (Math|Vector|MakeVector _returnvalue_3 _returnvalue_3 1.0))
    (else
      (Components|DestroyComponent (Variables|Default|GetContact%20Shadow)))))