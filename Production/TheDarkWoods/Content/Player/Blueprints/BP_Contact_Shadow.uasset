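; BP_Contact_Shadow is a contact shadow mesh that follows the ground beneath its parent actor.
; Each Tick it line-traces straight down a short distance from the parent actor's location against WorldStatic and WorldDynamic objects.
; On a hit, the static mesh eases toward the impact location with VInterpTo; without a hit it is not repositioned.
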(event EventBeginPlay)

(event Collision|EventActorBeginOverlap
  (params (OtherActor :type Actor%20Object%20Reference)))

(event EventTick
  (params (DeltaSeconds :type Float%20%28single-precision%29))
  (bind _staticmeshcomponent (Variables|Debug|GetStaticMeshComponent))
  (bind _staticmeshcomponent_2 (Variables|Debug|GetStaticMeshComponent))
  (bind _returnvalue (Components|GetOwner _staticmeshcomponent))
  (bind _returnvalue_2 (Actor|GetParentActor _returnvalue))
  (bind _returnvalue_3 (Transformation|GetActorLocation _returnvalue_2))
  (bind (_outhit _returnvalue_4) (Collision|LineTraceForObjects _returnvalue_3 (+ _returnvalue_3 (* "0, 0,1.000000" -3e+02)) (Utilities|Array|MakeArray "ObjectTypeQuery1" "ObjectTypeQuery2") false 0 "None"))
  (if _returnvalue_4
    (Transformation|SetWorldLocation _staticmeshcomponent_2 (Math|Interpolation|VInterpTo (Transformation|GetWorldLocation _staticmeshcomponent_2) (.location _outhit) (Utilities|Time|GetWorldDeltaSeconds) 3.0) false false)))

(fn ConstructionScript)