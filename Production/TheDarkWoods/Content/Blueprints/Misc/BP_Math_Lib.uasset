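; Blueprint math library of small helper functions for vector and scalar operations.
; GetVectorXY zeroes a vector's Z and returns the flat vector along with normalized and scaled versions.
; Scalar helpers negate a value, clamp it to the 0–1 range, or add to a variable in place by reference.
; Despite its name, OneMinus multiplies its input by one, returning it unchanged instead of subtracting it from one.
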(fn GetVectorXY
  (params (Vector :type Vector) (Scale :type Float%20%28single-precision%29))
  (bind _returnvalue (Math|Vector|MakeVector (.x Vector) (.y Vector) 0.0))
  (bind _returnvalue_2 (Math|Vector|Normalize _returnvalue))
  (return _returnvalue _returnvalue_2 (* _returnvalue_2 Scale)))

(fn OneMinus
  (params (x :type Float%20%28single-precision%29))
  (return (* 1.0 x)))

(fn Invert
  (params (x :type Float%20%28single-precision%29))
  (return (* x -1.0)))

(fn +=
  (params (A :type Float%20%28single-precision%29%20%28by%20ref%29) (B :type Float%20%28single-precision%29))
  (|SetBy-RefVar A (+ A B)))

(fn Clamp01
  (params (Value :type Float%20%28single-precision%29))
  (return (Math|Float|Clamp(Float) Value)))