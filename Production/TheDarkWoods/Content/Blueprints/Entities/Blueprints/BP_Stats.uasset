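; BP_Stats is an entity stats Blueprint that computes the damage one stat set deals to another.
; AttackOther sums CalculateNewAP across Base, Magic, Explosive, Fire and Ice, using own Attack against the target's Defence and Resistance.
; Each type scales Attack by resistance, capped at 100, then subtracts Defence unclamped.
; The resistance division precedes float conversion, apparently truncating fractional multipliers.
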(event EventBeginPlay)

(event EventTick
  (params (DeltaSeconds :type Float%20%28single-precision%29)))

(fn CalculateNewAP
  (params (Attack :type Integer) (Defence :type Integer) (Resistance :type Integer))
  (return (- (* (Math|Conversions|ToFloat(Integer) Attack) (Math|Conversions|ToFloat(Integer) (/ (- 100 (Math|Integer|Min(Integer) Resistance 100)) 100))) (Math|Conversions|ToFloat(Integer) Defence))))

(fn AttackOther
  (params (Target :type BP%20Stats%20Object%20Reference))
  (bind _attack (Variables|Default|GetAttack))
  (bind _defence (Variables|BP_Stats_C|GetDefence Target))
  (bind _resistance (Variables|BP_Stats_C|GetResistance Target))
  (return (+ (CallFunction|CalculateNewAP (.base _attack) (.base _defence) (.base _resistance)) (CallFunction|CalculateNewAP (.magic _attack) (.magic _defence) (.magic _resistance)) (CallFunction|CalculateNewAP (.explosive _attack) (.explosive _defence) (.explosive _resistance)) (CallFunction|CalculateNewAP (.fire _attack) (.fire _defence) (.fire _resistance)) (CallFunction|CalculateNewAP (.ice _attack) (.ice _defence) (.ice _resistance)))))