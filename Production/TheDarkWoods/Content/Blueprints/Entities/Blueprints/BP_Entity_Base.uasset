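; BP_Entity_Base is a base entity with combat stats, hit points and an optional contact shadow.
; The construction script fits the shadow to capsule and mesh bounds, and totals attack and defence points across damage types.
; AttackOther compares both entities' stats and charges the result to the target's HitPoints, which destroys the actor when empty.
; It also offers stat, status effect and closest-actor lookups, though status effect calculation is an empty stub.
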(event EventBeginPlay)

(event Collision|EventActorBeginOverlap
  (params (OtherActor :type Actor%20Object%20Reference)))

(event EventTick
  (params (DeltaSeconds :type Float%20%28single-precision%29)))

(fn ConstructionScript
  (bind _contact_shadow (Variables|ContactShadow|GetContact%20Shadow))
  (bind _contact_shadow_multiplier (Variables|ContactShadow|GetContact%20Shadow%20Multiplier))
  (bind _mesh (Variables|Character|GetMesh))
  (bind _boxextent (Collision|GetComponentBounds _mesh))
  (bind _relativelocation (Variables|/Script/Engine.SceneComponent|GetRelativeLocation _contact_shadow))
  (bind _returnvalue (Math|Float|Max(Float) (.x _boxextent) (.y _boxextent)))
  (bind _returnvalue_2 (/ _returnvalue 1e+02))
  (bind _returnvalue_3 (* _returnvalue_2 _contact_shadow_multiplier))
  (Utilities|FlowControl|Sequence
    (:then_0
      (if (Variables|ContactShadow|GetUse%20Contact%20Shadow?)
        ;[1 0.4333 0.9431] Init contact shadow
        (Transformation|SetRelativeLocation _contact_shadow (Math|Vector|MakeVector (.x _relativelocation) (.y _relativelocation) (+ (- (CallFunction|Invert (Components|Capsule|GetScaledCapsuleHalfHeight (Variables|Collision|GetCapsuleComponent))) 5e+01) (Variables|ContactShadow|GetContact%20Shadow%20Z%20Offset))) false false)
        (Transformation|SetWorldScale3D (Variables|ContactShadow|GetContact%20Shadow) (Math|Vector|MakeVector _returnvalue_3 _returnvalue_3 1.0))
        (else
          (Components|DestroyComponent (Variables|ContactShadow|GetContact%20Shadow)))))
    (:then_1
      (Utilities|FlowControl|Sequence
        (:then_0
          (Variables|Attributes|SetTotal%20Attack%20Points 0.0)
          (bind _damage (Utilities|ForEachDamageType (.Stat (Attributes|GetStat "NewEnumerator0")))
            (:LoopBody
              (Variables|Attributes|SetTotal%20Attack%20Points (+ (Variables|Attributes|GetTotal%20Attack%20Points) _damage)))))
        (:then_1
          (Variables|Attributes|SetTotal%20Defence%20Points 0.0)
          (bind _damage_2 (Utilities|ForEachDamageType (.Stat (Attributes|GetStat "NewEnumerator1")))
            (:LoopBody
              (Variables|Attributes|SetTotal%20Defence%20Points (+ (Variables|Attributes|GetTotal%20Defence%20Points) _damage_2)))))))))

(fn GetStatusEffectsList
  (return (Actor|GetComponentsByClass "/Game/Blueprints/Entities/Blueprints/BP_StatusEffect.BP_StatusEffect_C")))

(fn CalcStatusEffects)

(fn PopulateStats
  (CallFunction|PopulateStats (Variables|Attributes|GetStats) 0.0))

(fn AttackOther
  (params (Other :type BP%20Entity%20Base%20Object%20Reference))
  (bind _attack_points (CallFunction|CalculateAttack (Attributes|GetStats) (Attributes|GetStats Other)))
  (Development|PrintString (Utilities|String|Append "AP: " (Utilities|String|ToString(Float) _attack_points)))
  (Default|AddCost (Variables|BP_Entity_Base_C|GetHit%20Points Other) _attack_points))

(fn GetStats
  (return (Variables|Attributes|GetStats)))

(fn GetStat
  (params (Stat%20Type :type EStatType%20Enum :default "NewEnumerator0"))
  (bind _stats (Variables|Attributes|GetStats))
  (bind (_value _returnvalue) (Utilities|Map|Find (.stats _stats) Stat%20Type))
  (return _value _returnvalue))

(fn GetDamage
  (params (Stat :type F%20Single%20Stat%20Structure) (Damage%20Type :type EDamageType%20Enum :default "NewEnumerator0"))
  (bind _damagetype (Utilities|Struct|BreakFSingleStat Stat))
  (bind (_value _returnvalue) (Utilities|Map|Find _damagetype Damage%20Type))
  (return _value _returnvalue))

(fn GetStatDamage
  (params (Stat%20Type :type EStatType%20Enum :default "NewEnumerator0") (Damage%20Type :type EDamageType%20Enum :default "NewEnumerator0"))
  (return (.Damage (Attributes|GetDamage (.Stat (Attributes|GetStat Stat%20Type)) Damage%20Type))))

(fn GetClosestActor
  (params (ActorClass :type Actor%20Class%20Reference) (Query%20Distance? :type Boolean) (Query%20Distance :type Float%20%28single-precision%29))
  (bind _outactors (Actor|GetAllActorsOfClass ActorClass))
  (for _array_element _outactors
    (if (< (Transformation|GetDistanceTo _array_element) (LocalVariables|GetClosest%20Distance))
      _
      (else
        (Utilities|FlowControl|DoOnce false
          (:Completed
            _))))
    (LocalVariables|SetClosest%20Distance (Transformation|GetDistanceTo _array_element))
    (LocalVariables|SetClosest%20Actor _array_element))
  (if Query%20Distance?
    (if (<= (LocalVariables|GetClosest%20Distance) Query%20Distance)
      _
      (else
        (return 0 (LocalVariables|GetClosest%20Distance)))))
  (return (LocalVariables|GetClosest%20Actor) (LocalVariables|GetClosest%20Distance)))

(event OnEmpty(HitPoints)
  (CallFunction|Kill))

(event Custom|Kill
  (Utilities|FlowControl|DoOnce false
    (:Completed
      (Default|SetValue (Variables|Attributes|GetHit%20Points) 0.0)
      (Actor|DestroyActor))))