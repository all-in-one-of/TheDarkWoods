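; Status effect component that lasts for a set Duration, then destroys itself through a one-shot timer started on BeginPlay.
; SetDuration clears the stored timer and starts another, using either the full new duration or the elapsed time minus that duration, clamped at zero.
; The elapsed time is read after the clear, and the replacement timer's handle is not stored.
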(event Custom|Destroy
  (Components|DestroyComponent))

(event Custom|SetDuration
  (params (Duration :type Float%20%28single-precision%29) (Reset%20Timer :type Boolean))
  ;[1 1 1] Set duration & handle timer according to new time
  (bind _output_get (Variables|Default|SetDuration Duration))
  (Utilities|Time|ClearandInvalidateTimerbyHandle (stale EventBeginPlay _returnvalue))
  (Utilities|Time|SetTimerbyEvent (delegate Custom|Destroy) (Math|Float|SelectFloat _output_get (Math|Float|Max(Float) (- (Class|KismetSystemLibrary|GetTimerElapsedTimeHandle (stale EventBeginPlay _returnvalue)) Duration) 0.0) Reset%20Timer)))

(event EventBeginPlay
  ;[1 0.6824 0.1812] Init
  (bind _returnvalue (Utilities|Time|SetTimerbyEvent (delegate Custom|Destroy) (Variables|Default|GetDuration))))