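; BP_Attribute is a reusable bounded integer attribute that tracks a current value against a maximum.
; SetValue clamps the new value between zero and MaxValue, then dispatches OnEmpty or OnFull when it sits at either limit, with empty taking priority.
; IsEmpty and IsFull expose those limit checks as functions.
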(event Custom|SetValue
  (params (Value :type Integer))
  (Utilities|FlowControl|Sequence
    (:then_0
      (Variables|Default|SetValue (Math|Integer|Clamp(Integer) Value 0 (Variables|Default|GetMax%20Value))))
    (:then_1
      ;[1 0.3393 0.08707] OnEmpty and OnFull event dispatch handling
      (if (CallFunction|IsEmpty)
        (Default|CallOnEmpty)
        (elif (CallFunction|IsFull)
          (Default|CallOnFull))))))

(event EventBeginPlay)

(event EventTick
  (params (DeltaSeconds :type Float%20%28single-precision%29)))

(fn IsEmpty
  (return (<= (Variables|Default|GetValue) 0)))

(fn IsFull
  (return (>= (Variables|Default|GetValue) (Variables|Default|GetMax%20Value))))