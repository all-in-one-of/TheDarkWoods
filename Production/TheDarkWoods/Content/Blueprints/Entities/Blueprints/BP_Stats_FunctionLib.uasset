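; Blueprint function library for combat stats stored as nested maps of stat type and damage type.
; Populate functions loop the enums to add missing map entries; a comment flags the nested single-stat call in PopulateStats as broken.
; CalculateAttack applies CalculateAttackOnStat per damage type, subtracting resistance-scaled attack from defence, and returns per-type results plus their sum.
; Negative results mean damage; resistance caps at 100, with negative values amplifying attack.
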(fn PopulateSingleStat
  (params (Stat :type F%20Single%20Stat%20Structure%20%28by%20ref%29) (Default :type Float%20%28single-precision%29))
  (bind _output_get (LocalVariables|SetBuffer (|Copy Stat)))
  (bind _enumvalue (|ForEachEDamageType)
    (:LoopBody
      (if (not (.ReturnValue (Utilities|Map|Find (Utilities|Struct|BreakFSingleStat _output_get) _enumvalue)))
        (Utilities|Map|Add (Utilities|Struct|BreakFSingleStat _output_get) _enumvalue Default)))
    (:then
      (|SetBy-RefVar Stat (LocalVariables|GetBuffer))
      (return Stat))))

(fn PopulateStats
  (params (Stats :type F%20Stats%20Structure%20%28by%20ref%29) (Default :type Float%20%28single-precision%29))
  (bind _output_get (LocalVariables|SetBuffer (|Copy Stats)))
  (bind _enumvalue (|ForEachEStatType)
    (:LoopBody
      (if (not (.ReturnValue (Utilities|Map|Find (Utilities|Struct|BreakFStats _output_get) _enumvalue)))
        (Utilities|Map|Add (Utilities|Struct|BreakFStats _output_get) _enumvalue (.Value (Utilities|Map|Find (Utilities|Struct|BreakFStats _output_get) _enumvalue)))
        (Attributes|Stats|Populate|PopulateSingleStat (.Value (Utilities|Map|Find (Utilities|Struct|BreakFStats _output_get) _enumvalue)) Default (LocalVariables|Get__WorldContext)) ; BROKEN WHEN USED HERE
      ))
    (:then
      (|SetBy-RefVar Stats (LocalVariables|GetBuffer)))))

(fn CalculateAttackonStat
  (params (Attack :type Float%20%28single-precision%29%20%28by%20ref%29) (Defence :type Float%20%28single-precision%29%20%28by%20ref%29) (Resistance :type Float%20%28single-precision%29%20%28by%20ref%29))
  (return (- Defence (* Attack (/ (- 1e+02 (Math|Float|Min(Float) Resistance 1e+02)) 1e+02)))))

(fn CalculateAttack
  (params (Attacker%20Stats :type F%20Stats%20Structure) (Defender%20Stats :type F%20Stats%20Structure))
  (bind _stats (Utilities|Struct|BreakFStats Defender%20Stats))
  (bind _enumvalue (|ForEachEDamageType)
    (:LoopBody
      (Utilities|Map|Add (Utilities|Struct|BreakFSingleStat (LocalVariables|GetResult)) _enumvalue (Attributes|Stats|CalculateAttackonStat (.Value (Utilities|Map|Find (.damagetype (.Value (Utilities|Map|Find (Utilities|Struct|BreakFStats Attacker%20Stats) "NewEnumerator0"))) _enumvalue)) (.Value (Utilities|Map|Find (.damagetype (.Value (Utilities|Map|Find _stats "NewEnumerator1"))) _enumvalue)) (.Value (Utilities|Map|Find (.damagetype (.Value (Utilities|Map|Find _stats "NewEnumerator2"))) _enumvalue)) (LocalVariables|Get__WorldContext)))
      (LocalVariables|SetFloat%20Result (+ (LocalVariables|GetFloat%20Result) (Attributes|Stats|CalculateAttackonStat (.Value (Utilities|Map|Find (.damagetype (.Value (Utilities|Map|Find (Utilities|Struct|BreakFStats Attacker%20Stats) "NewEnumerator0"))) _enumvalue)) (.Value (Utilities|Map|Find (.damagetype (.Value (Utilities|Map|Find _stats "NewEnumerator1"))) _enumvalue)) (.Value (Utilities|Map|Find (.damagetype (.Value (Utilities|Map|Find _stats "NewEnumerator2"))) _enumvalue)) (LocalVariables|Get__WorldContext)))))
    (:then
      (return (LocalVariables|GetFloat%20Result) (LocalVariables|GetResult)))))