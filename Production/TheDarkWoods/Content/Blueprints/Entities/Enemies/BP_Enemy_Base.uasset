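; Base enemy Blueprint with an overhead stats widget and player-facing aggro behavior.
; The construction script places the widget above the mesh bounds plus an offset; BeginPlay sets the enemy as the widget's owner, and Tick billboards it to the camera.
; While the player overlaps AggroRadius, the enemy smoothly yaws toward them.
; Entering the radius shows the widget, and leaving hides it after a delay.
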(event OnComponentBeginOverlap(AggroRadius)
  (params (OverlappedComponent :type Primitive%20Component%20Object%20Reference) (OtherActor :type Actor%20Object%20Reference) (OtherComp :type Primitive%20Component%20Object%20Reference) (OtherBodyIndex :type Integer) (bFromSweep :type Boolean) (SweepResult :type Hit%20Result%20Structure%20%28by%20ref%29))
  (if (== OtherActor (Game|Player|GetPlayerPawn 0))
    (Rendering|SetVisibility (Variables|Default|GetStats%20Widget) true false)))

(event OnComponentEndOverlap(AggroRadius)
  (params (OverlappedComponent :type Primitive%20Component%20Object%20Reference) (OtherActor :type Actor%20Object%20Reference) (OtherComp :type Primitive%20Component%20Object%20Reference) (OtherBodyIndex :type Integer))
  (if (== OtherActor (Game|Player|GetPlayerPawn 0))
    (Utilities|FlowControl|Delay (Variables|Attributes|GetStats%20Widget%20Duration))
    (Rendering|SetVisibility (Variables|Default|GetStats%20Widget) false false)))

(event EventBeginPlay
  (|CallParentFunction)
  ;[1 0.4267 0.1633] Init stats widget
  (bind _asbp_ui_enemy_stats (Utilities|Casting|CastToBP_UI_EnemyStats (UserInterface|GetUserWidgetObject (Variables|Default|GetStats%20Widget))))
  (Variables|/Game/UI/Blueprints/BP_UI_EnemyStats.BP_UI_EnemyStats_C|SetOwner _asbp_ui_enemy_stats self))

(event Collision|EventActorBeginOverlap
  (params (OtherActor :type Actor%20Object%20Reference))
  (|CallParentFunction OtherActor))

(event EventTick
  (params (DeltaSeconds :type Float%20%28single-precision%29))
  (bind _returnvalue (Game|Player|GetPlayerPawn 0))
  (bind _returnvalue_2 (Transformation|GetActorRotation))
  (bind _stats_widget (Variables|Default|GetStats%20Widget))
  (bind (_roll _pitch) (Math|Rotator|BreakRotator _returnvalue_2))
  (|CallParentFunction DeltaSeconds)
  (Utilities|FlowControl|Sequence
    (:then_0
      ;[0.6146 1 0.2292] Billboard stats widget
      (Transformation|SetWorldRotation _stats_widget (Math|Rotator|FindLookatRotation (Transformation|GetWorldLocation _stats_widget) (Transformation|GetActorLocation (Game|GetPlayerCameraManager 0))) false false))
    (:then_1
      (if (Collision|IsOverlappingActor (Variables|Default|GetAggro%20Radius) _returnvalue :!class /Script/Engine.PrimitiveComponent)
        (Transformation|SetActorRotation (Math|Rotator|MakeRotator _roll _pitch (.yaw (Math|Interpolation|RInterpTo _returnvalue_2 (Math|Rotator|FindLookatRotation (Transformation|GetActorLocation) (Transformation|GetActorLocation _returnvalue)) (Utilities|Time|GetWorldDeltaSeconds) 3.0))))))))

(fn ConstructionScript
  (bind _mesh (Variables|Character|GetMesh))
  (bind _stats_widget (Variables|Default|GetStats%20Widget))
  (bind _returnvalue (Transformation|GetWorldLocation _stats_widget))
  (bind (_origin _boxextent) (Collision|GetComponentBounds _mesh))
  (|CallParentFunction)
  (Transformation|SetWorldLocation _stats_widget (Math|Vector|MakeVector (.x _returnvalue) (.y _returnvalue) (+ (.z _origin) (.z _boxextent) (Variables|Attributes|GetStats%20Widget%20Z%20Offset))) false false))