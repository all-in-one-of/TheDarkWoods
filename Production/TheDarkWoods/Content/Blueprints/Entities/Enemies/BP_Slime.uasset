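; BP_Slime is a slime enemy Blueprint that gives each instance a varied look.
; Its construction script picks a random body material, scales the mesh randomly per axis and shares one dynamic eye material between both eyes, driven by EyeIndex.
; A separate Randomise function rerolls EyeIndex but is not called within this graph.
; BeginPlay offsets the mesh animation to a random position so nearby slimes animate out of sync.
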(event EventBeginPlay
  (|CallParentFunction)
  ;[1 1 1] Randomise animation to prevent nearby slimes being in sync
  (Components|Animation|SetPosition (Variables|Character|GetMesh) (Math|Random|RandomFloatinRange 0.0 1.0) false))

(event Collision|EventActorBeginOverlap
  (params (OtherActor :type Actor%20Object%20Reference))
  (|CallParentFunction OtherActor))

(event EventTick
  (params (DeltaSeconds :type Float%20%28single-precision%29))
  (|CallParentFunction DeltaSeconds))

(fn ConstructionScript
  (bind _returnvalue (Math|Random|RandomFloatinRange 0.5 1.0))
  (bind _random_materials (Variables|Default|GetRandom%20Materials))
  (|CallParentFunction)
  (Utilities|FlowControl|Sequence
    (:then_0
      (Rendering|Material|SetMaterial (Variables|Character|GetMesh) 0 (Utilities|Array|Get(acopy) _random_materials (Math|Random|RandomIntegerinRange 0 (Utilities|Array|LastIndex _random_materials)))))
    (:then_1
      (bind _returnvalue_2 (Rendering|Material|CreateDynamicMaterialInstance (Variables|Default|GetEyeL) 0 "/Game/Assets/Enemies/Materials/MI_Slime_Eyes.MI_Slime_Eyes" :!class /Script/Engine.PrimitiveComponent))
      (Rendering|Material|SetMaterial (Variables|Default|GetEyeR) 0 _returnvalue_2)
      (Rendering|Material|SetScalarParameterValue _returnvalue_2 "Index" (Variables|Default|GetEye%20Index) :!class /Script/Engine.MaterialInstanceDynamic))
    (:then_2
      (Transformation|SetWorldScale3D (Variables|Character|GetMesh) (Math|Vector|MakeVector _returnvalue _returnvalue _returnvalue)))))

(fn Randomise
  (Variables|Default|SetEye%20Index (Math|Random|RandomFloatinRange 0.0 1.0)))