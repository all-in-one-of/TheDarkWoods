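; BP_Boolean is an actor that publishes a spherical boolean volume to materials through the SPC_Boolean parameter collection.
; Construct writes the actor's location and Radius into the collection's position and radius parameters, then sizes the Sphere component to the same Radius.
; It runs from the construction script and again on BeginPlay, with no per-frame update.
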(event EventBeginPlay
  (CallFunction|Construct))

(event Collision|EventActorBeginOverlap
  (params (OtherActor :type Actor%20Object%20Reference)))

(event EventTick
  (params (DeltaSeconds :type Float%20%28single-precision%29)))

(fn ConstructionScript
  (CallFunction|Construct))

(fn Construct
  (bind _radius (Variables|Default|GetRadius))
  (Utilities|FlowControl|Sequence
    (:then_0
      (Rendering|Material|SetVectorParameterValue "/Game/Assets/Shaders/Boolean/SPC_Boolean.SPC_Boolean" "Boolean Position" (Math|Conversions|ToLinearColor(Vector) (Transformation|GetActorLocation)) :!class /Script/Engine.KismetMaterialLibrary))
    (:then_1
      (Rendering|Material|SetScalarParameterValue "/Game/Assets/Shaders/Boolean/SPC_Boolean.SPC_Boolean" "Boolean Radius" _radius :!class /Script/Engine.KismetMaterialLibrary))
    (:then_2
      (Components|Sphere|SetSphereRadius (Variables|Default|GetSphere) _radius false))))