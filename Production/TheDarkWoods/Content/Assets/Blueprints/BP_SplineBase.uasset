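; Base spline actor, by its name a parent for other spline Blueprints, with utilities for copying and retyping spline points.
; Construct runs from the construction script and, if ForcePointType is set, applies PointType to all points, optionally excluding endpoints.
; StealPoints rebuilds the spline from another actor's first spline component, saving undo state first.
; SetPointsToType retypes every point when forcing is off, sharing the ForEachSplinePoint macro and RefreshSpline.
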(event EventBeginPlay
  (|CallParentFunction))

(fn ConstructionScript
  (|CallParentFunction)
  (Spline|Utility|Construct))

(fn StealPoints
  (bind _spline (Variables|Default|GetSpline))
  (bind _steal_points_from_actor (Variables|Spline|GetSteal%20Points%20From%20Actor))
  (bind _returnvalue (Actor|GetComponentsByClass _steal_points_from_actor "/Script/Engine.SplineComponent"))
  (bind _output (Utilities|Array|Get(acopy) _returnvalue))
  (bind _returnvalue_2 (Spline|GetNumberOfSplinePoints _output))
  (bind _returnvalue_3 (- _returnvalue_2 1))
  ;[1 1 1] If there is a spline to steal from
  (if (!= (Variables|Spline|GetSteal%20Points%20From%20Actor) 0)
    (if (!= _output 0)
      (Development|Editor|CreateCopyforUndoBuffer self)
      (Utilities|FlowControl|Sequence
        (:then_0
          (Spline|ClearSplinePoints (Variables|Default|GetSpline) true)
          (for _index (range (Class|KismetSystemLibrary|MakeLiteralInteger) _returnvalue_3)
            (Utilities|FlowControl|Sequence
              (:then_0
                (Spline|AddSplinePoint _spline (Spline|GetLocationatSplinePoint _output _returnvalue_3 "Local") "Local" false))
              (:then_1
                (Spline|SetSplinePointType _spline _returnvalue_3 (Class|SplineComponent|GetSplinePointType _output _returnvalue_3) false))
              (:then_2
                (Spline|SetTangentatSplinePoint _spline _returnvalue_3 (Spline|GetTangentatSplinePoint _output _returnvalue_3 "Local") "Local" false))
              (:then_3
                (Spline|SetTangentsatSplinePoint _spline _returnvalue_3 (Spline|GetArriveTangentatSplinePoint _output _returnvalue_3 "Local") (Spline|GetLeaveTangentatSplinePoint _output _returnvalue_3 "Local") "Local" false))
              (:then_4
                (Class|SplineComponent|SetUpVectoratSplinePoint _spline _returnvalue_3 (Class|SplineComponent|GetUpVectoratSplinePoint _output 0 "Local") "Local" false)))))
        (:then_1
          (Spline|Utility|RefreshSpline true))))))

(fn Construct
  (bind _force_end_point_types_ (Variables|Spline|PointType|GetForce%20End%20Point%20Types?))
  (Utilities|FlowControl|Sequence
    (:then_0
      (if (Variables|Spline|PointType|GetForce%20Point%20Type?)
        (bind (_spline _index) (Utilities|ForEachSplinePoint (Math|Integer|SelectInt 0 1 _force_end_point_types_) (Math|Integer|SelectInt 1 2 _force_end_point_types_))
          (:LoopBody
            (Spline|SetSplinePointType _spline _index (Variables|Spline|PointType|GetPoint%20Type) false))
          (:Completed
            (Spline|UpdateSpline _spline)))))
    (:then_1
      (return true))))

(fn SetPointstoType
  (if (not (Variables|Spline|PointType|GetForce%20Point%20Type?))
    (bind (_spline _index) (Utilities|ForEachSplinePoint 0 1)
      (:LoopBody
        (Spline|SetSplinePointType _spline _index (Variables|Spline|PointType|GetPoint%20Type) false))
      (:Completed
        (Spline|Utility|RefreshSpline true)))))

(fn RefreshSpline
  (params (Construct :type Boolean))
  (Spline|UpdateSpline (Variables|Default|GetSpline))
  (if Construct
    (Spline|Utility|Construct))
  (return true))

(fn ReconstructSpline
  (Spline|Utility|RefreshSpline true))