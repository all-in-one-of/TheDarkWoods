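; Spline path actor that snaps its spline points to the surface below in its overridden Construct function.
; Each point gets a downward object-type line trace from the actor's height plus ZOffset, with debug drawing.
; Hit points move to the impact plus ZOffset without an immediate spline update, then the parent Construct runs.
; Tangent adjustment nodes are left unconnected, and the event graph holds no active logic.
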(event EventBeginPlay
  (|CallParentFunction))

(event Collision|EventActorBeginOverlap
  (params (OtherActor :type Actor%20Object%20Reference))
  (|CallParentFunction OtherActor))

(event EventTick
  (params (DeltaSeconds :type Float%20%28single-precision%29))
  (|CallParentFunction DeltaSeconds))

(fn ConstructionScript
  (|CallParentFunction))

(fn Construct
  (Utilities|FlowControl|Sequence
    (:then_0
      (for _index (range (Class|KismetSystemLibrary|MakeLiteralInteger) (- (Spline|GetNumberOfSplinePoints (Variables|Default|GetSpline)) 1))
        (bind (_outhit _returnvalue) (Collision|LineTraceForObjects (Math|Vector|MakeVector (.x (Spline|GetLocationatSplinePoint (Variables|Default|GetSpline) _index "World")) (.y (Spline|GetLocationatSplinePoint (Variables|Default|GetSpline) _index "World")) (+ (.z (Transformation|GetActorLocation)) (Variables|SplineMesh|Trace|GetZ%20Offset))) (+ (Math|Vector|MakeVector (.x (Spline|GetLocationatSplinePoint (Variables|Default|GetSpline) _index "World")) (.y (Spline|GetLocationatSplinePoint (Variables|Default|GetSpline) _index "World")) (+ (.z (Transformation|GetActorLocation)) (Variables|SplineMesh|Trace|GetZ%20Offset))) (Math|Vector|MakeVector 0.0 0.0 (CallFunction|Invert (Variables|SplineMesh|Trace|GetTrace%20Distance)))) (Variables|SplineMesh|Trace|GetTrace%20Types) (Variables|SplineMesh|Trace|GetTrace%20Complex?) 0 "ForDuration" true "(R=1.000000,G=0.000000,B=0.000000,A=1.000000)" "(R=0.000000,G=1.000000,B=0.000000,A=1.000000)" 0.25))
        (if _returnvalue
          (Utilities|FlowControl|Sequence
            (:then_0
              (Spline|SetLocationatSplinePoint (Variables|Default|GetSpline) _index (+ (.location _outhit) (Math|Vector|MakeVector 0.0 0.0 (Variables|SplineMesh|Trace|GetZ%20Offset))) "World" false))))))
    (:then_1
      (bind _successful (|CallParentFunction))
      (return _successful))))