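; Spline tree actor that bends a single spline mesh along the first two points of its spline.
; Its Construct override calls the parent, then copies both points' local locations and tangents into the mesh.
; Both point scales go to the mesh's end scale, so the second overwrites the first and start scale is never set.
; The event graph holds only disabled stubs.
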(event EventBeginPlay)

(event Collision|EventActorBeginOverlap
  (params (OtherActor :type Actor%20Object%20Reference)))

(event EventTick
  (params (DeltaSeconds :type Float%20%28single-precision%29)))

(fn ConstructionScript
  (|CallParentFunction))

(fn Construct
  (bind _spline (Variables|Default|GetSpline))
  (bind _splinemesh (Variables|Default|GetSplineMesh))
  (bind (_location _tangent) (Spline|GetLocationandTangentatSplinePoint _spline 1 "Local"))
  (bind (_location_2 _tangent_2) (Spline|GetLocationandTangentatSplinePoint _spline 0 "Local"))
  (|CallParentFunction)
  (Utilities|FlowControl|Sequence
    (:then_0
      (SplineMesh|SetStartandEnd _splinemesh _location_2 _tangent_2 _location _tangent false :!class /Script/Engine.SplineMeshComponent))
    (:then_1
      (SplineMesh|SetEndScale _splinemesh (Math|Conversions|ToVector2D(Vector) (Spline|GetScaleatSplinePoint _spline 0)) false :!class /Script/Engine.SplineMeshComponent)
      (SplineMesh|SetEndScale _splinemesh (Math|Conversions|ToVector2D(Vector) (Spline|GetScaleatSplinePoint _spline 1)) true :!class /Script/Engine.SplineMeshComponent))
    (:then_2
      (return true))))