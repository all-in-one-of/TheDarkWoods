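; Wind controller actor that pushes global wind settings for foliage materials into the SPC_Wind Material Parameter Collection.
; UpdateWind writes the actor's forward vector as the wind direction, along with its Tiling, Intensity and Speed variables.
; It runs from the construction script and again on BeginPlay, so rotating or editing the actor updates the wind in the editor; there is no per-frame update.
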(event EventBeginPlay
  (CallFunction|UpdateWind))

(event Collision|EventActorBeginOverlap
  (params (OtherActor :type Actor%20Object%20Reference)))

(event EventTick
  (params (DeltaSeconds :type Float%20%28single-precision%29)))

(fn ConstructionScript
  (CallFunction|UpdateWind))

(fn UpdateWind
  (Utilities|FlowControl|Sequence
    (:then_0
      (Rendering|Material|SetVectorParameterValue "/Game/Assets/Foliage/Materials/SPC_Wind.SPC_Wind" "Direction" (Math|Conversions|ToLinearColor(Vector) (Transformation|GetActorForwardVector)) :!class /Script/Engine.KismetMaterialLibrary))
    (:then_1
      (Rendering|Material|SetScalarParameterValue "/Game/Assets/Foliage/Materials/SPC_Wind.SPC_Wind" "Tiling" (Variables|Wind|GetTiling) :!class /Script/Engine.KismetMaterialLibrary)
      (Rendering|Material|SetScalarParameterValue "/Game/Assets/Foliage/Materials/SPC_Wind.SPC_Wind" "Intensity" (Variables|Wind|GetIntensity) :!class /Script/Engine.KismetMaterialLibrary)
      (Rendering|Material|SetScalarParameterValue "/Game/Assets/Foliage/Materials/SPC_Wind.SPC_Wind" "Speed" (Variables|Wind|GetSpeed) :!class /Script/Engine.KismetMaterialLibrary))))