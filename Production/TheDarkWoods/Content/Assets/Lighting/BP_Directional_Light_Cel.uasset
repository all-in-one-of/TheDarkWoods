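; Directional light Blueprint that publishes its settings as global material parameters for cel shading.
; UpdateCel writes the actor's forward vector to "Cel Light Direction" in the SPC_General parameter collection.
; It also writes "Cel Light Colour", packing light colour into RGB and intensity into alpha.
; The update runs in the construction script and on BeginPlay, with no per-frame refresh.
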(event EventBeginPlay
  (CallFunction|UpdateCel))

(event EventTick
  (params (DeltaSeconds :type Float%20%28single-precision%29)))

(fn ConstructionScript
  (CallFunction|UpdateCel))

(fn UpdateCel
  (bind _lightcomponent (Variables|Default|GetLightComponent))
  (bind _returnvalue (Rendering|Components|Light|GetLightColor _lightcomponent))
  (Utilities|FlowControl|Sequence
    (:then_0
      (Rendering|Material|SetVectorParameterValue "/Game/Assets/Shaders/SPC_General.SPC_General" "Cel Light Direction" (Math|Conversions|ToLinearColor(Vector) (Math|Vector|GetForwardVector (Transformation|GetActorRotation))) :!class /Script/Engine.KismetMaterialLibrary))
    (:then_1
      (Rendering|Material|SetVectorParameterValue "/Game/Assets/Shaders/SPC_General.SPC_General" "Cel Light Colour" (Utilities|Struct|MakeLinearColor (.r _returnvalue) (.g _returnvalue) (.b _returnvalue) (Variables|/Script/Engine.LightComponentBase|GetIntensity _lightcomponent)) :!class /Script/Engine.KismetMaterialLibrary))))