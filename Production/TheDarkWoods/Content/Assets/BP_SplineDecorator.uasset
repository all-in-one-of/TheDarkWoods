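; Spline decorator that scatters static mesh components along a spline, extending a parent Blueprint's construction.
; Construct steps along the spline by Density times local Z scale, picking from DecoratorMeshes via a random stream and sizing each by spline Y scale.
; Per-mesh and global transforms combine with random location, rotation and uniform-scale jitter, with relative or world space options for rotation.
; RandomiseSeed picks a new seed, destroys the SplineMeshes components and rebuilds.
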(event EventBeginPlay)

(event Collision|EventActorBeginOverlap
  (params (OtherActor :type Actor%20Object%20Reference)))

(event EventTick
  (params (DeltaSeconds :type Float%20%28single-precision%29)))

(fn ConstructionScript
  (|CallParentFunction))

(fn RandomiseSeed
  (Variables|SplineDecorator|SetSeed (Math|Random|RandomIntegerinRange 0 100000))
  (for _array_element (Variables|SplineDecorator|GetSpline%20Meshes)
    (Components|DestroyComponent _array_element))
  (CallFunction|Construct))

(fn GetRandomTransform
  (params (In :type F%20Randomised%20Transform%20Structure))
  (bind (_roll _pitch _yaw) (Math|Rotator|BreakRotator (.randomrotation In)))
  (bind _out (SplineDecorator|GetRandomVector (.randomlocation In)))
  (bind _returnvalue (Math|Transform|MakeTransform (.location In) (.rotation In)))
  (bind (_x _y) (Math|Vector2D|BreakVector2D (.randomuniformscalerange In)))
  (bind _stream (Variables|SplineDecorator|GetStream))
  (bind _returnvalue_2 (Math|Random|RandomFloatinRangefromStream _x _y _stream))
  (bind _out_2 (SplineDecorator|GetRandomVector (Math|Vector|MakeVector _roll _pitch _yaw)))
  (bind _returnvalue_3 (Math|Rotator|MakeRotator (.x _out_2) (.y _out_2) (.z _out_2)))
  (bind _returnvalue_4 (Math|Transform|MakeTransform _out _returnvalue_3 (Math|Vector|MakeVector _returnvalue_2 _returnvalue_2 _returnvalue_2)))
  (bind (_location _rotation _scale) (Math|Transform|BreakTransform _returnvalue_4))
  (return (Math|Transform|ComposeTransforms (Math|Transform|MakeTransform _location (Utilities|Select :Index (.randomtransformspace In) :NewEnumerator1 _rotation :NewEnumerator0 (.rotation (Math|Transform|ComposeTransforms _returnvalue_4 (Transformation|GetActorTransform)))) _scale) (Math|Transform|MakeTransform (.location _returnvalue) (.rotation _returnvalue) (* (.scale _returnvalue) (* (.scale In) (.uniformscale In)))))))

(fn GetRandomVector
  (params (In :type Vector))
  (bind _returnvalue (* In -1.0))
  (bind (_x _y _z) (Math|Vector|BreakVector In))
  (bind _stream (Variables|SplineDecorator|GetStream))
  (return (Math|Vector|MakeVector (Math|Random|RandomFloatinRangefromStream (.x _returnvalue) _x _stream) (Math|Random|RandomFloatinRangefromStream (.y _returnvalue) _y _stream) (Math|Random|RandomFloatinRangefromStream (.z _returnvalue) _z _stream))))

(fn CombineFTransforms
  (params (A :type F%20Randomised%20Transform%20Structure) (B :type F%20Randomised%20Transform%20Structure))
  (return (Utilities|Struct|MakeFRandomisedTransform (.transformspace A) (+ (.location A) (.location B)) (Math|Rotator|CombineRotators (.rotation A) (.rotation B)) (* (.scale A) (.scale B)) (* (.uniformscale A) (.uniformscale B)) (.randomtransformspace A) (+ (.randomlocation A) (.randomlocation B)) (Math|Rotator|CombineRotators (.randomrotation A) (.randomrotation B)) (* (.randomuniformscalerange A) (.randomuniformscalerange B)))))

(fn Construct
  (bind _spline (Variables|Default|GetSpline))
  (bind _stream (Variables|SplineDecorator|GetStream))
  (bind _decorator_meshes (Variables|SplineDecorator|GetDecorator%20Meshes))
  (bind _accum_distance (LocalVariables|GetAccum%20Distance))
  (bind _accum_distance_2 (LocalVariables|GetAccum%20Distance))
  (bind _returnvalue (Utilities|Array|LastIndex _decorator_meshes))
  (bind _returnvalue_2 (Spline|GetTransformatDistanceAlongSpline _spline _accum_distance "Local" true))
  (bind _returnvalue_3 (Math|Random|RandomIntegerinRangefromStream 0 _returnvalue _stream))
  (bind _output (Utilities|Array|Get(acopy) _decorator_meshes _returnvalue_3))
  (|CallParentFunction)
  (Utilities|FlowControl|Sequence
    (:then_0
      (while (<= (LocalVariables|GetAccum%20Distance) (Spline|GetSplineLength (Variables|Default|GetSpline)))
        (Utilities|FlowControl|Sequence
          (:then_0
            (bind _returnvalue_4 (AddComponent|AddStaticMeshComponent false (Math|Transform|ComposeTransforms (SplineDecorator|GetRandomTransform (SplineDecorator|CombineFTransforms (.transform _output) (Variables|SplineDecorator|GetGlobal%20Transform))) (Math|Transform|MakeTransform (.location _returnvalue_2) (Utilities|Select :Index (.splinespace _output) :NewEnumerator1 (.rotation _returnvalue_2) :NewEnumerator0 "0, 0, 0") (Math|Vector|MakeVector (.y (.scale _returnvalue_2)) (.y (.scale _returnvalue_2)) (.y (.scale _returnvalue_2)))))))
            (Utilities|FlowControl|Sequence
              (:then_0
                (Components|StaticMesh|SetStaticMesh _returnvalue_4 (.staticmesh _output))
                (Utilities|Array|Add (Variables|SplineDecorator|GetSpline%20Meshes) _returnvalue_4))))
          (:then_1
            (CallFunction|+= _accum_distance_2 (* (Variables|SplineDecorator|GetDensity) (.z (Class|SplineComponent|GetScaleatDistanceAlongSpline (Variables|Default|GetSpline) _accum_distance_2))))))))
    (:then_1
      (return true))))